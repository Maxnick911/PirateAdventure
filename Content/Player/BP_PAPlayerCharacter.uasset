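; Player character Blueprint that handles input for two attacks, a musket shot and a hook hit.
; Each press calls its attack function, which is not defined in this graph, then plays a non-looping animation on that weapon's mesh and a sound at the actor's location.
; A DoOnce per attack, reset after an animation delay variable, acts as a cooldown so each attack cannot retrigger mid-swing or mid-shot.
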(event EventBeginPlay)

(event Collision|EventActorBeginOverlap
  (params (OtherActor :type Actor%20Object%20Reference)))

(event EventTick
  (params (DeltaSeconds :type Float%20%28single-precision%29)))

(event Input|ActionEvents|InputActionHookHit
  (params (Key :type Key%20Structure :default "None"))
  (:Pressed
    (Utilities|FlowControl|DoOnce false :!label _label
      (:Completed
        (Class|PAPlayerCharacter|HookHit)
        (Components|Animation|PlayAnimation (Variables|Default|GetHookMesh) "/Game/Weapon/Hook/HookHitAnimation.HookHitAnimation" false)
        (Audio|PlaySoundatLocation "/Game/Weapon/Hook/HookHitSound.HookHitSound" (Transformation|GetActorLocation) "0, 0, 0" 1.0 1.0 0.0 0 0 0)
        (Utilities|FlowControl|Delay (Variables|Default|GetHookHitAnimationDelay))
        (goto _label Reset)))))

(event Input|ActionEvents|InputActionMusketShot
  (params (Key :type Key%20Structure :default "None"))
  (:Pressed
    (Utilities|FlowControl|DoOnce false :!label _label
      (:Completed
        (Class|PAPlayerCharacter|MusketShot)
        (Components|Animation|PlayAnimation (Variables|Default|GetMusketMesh) "/Game/Weapon/Musket/MusketShotAnimation.MusketShotAnimation" false)
        (Audio|PlaySoundatLocation "/Game/Weapon/Musket/MusketShotSound.MusketShotSound" (Transformation|GetActorLocation) "0, 0, 0" 1.0 1.0 0.0 0 0 0)
        (Utilities|FlowControl|Delay (Variables|Default|GetMusketShotAnimationDelay))
        (goto _label Reset)))))

(fn ConstructionScript)